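; Enemy spawner actor that creates escalating batches of enemies whenever the first-person game mode signals a respawn.
; It binds SpawnEnemy to the game mode on BeginPlay, then randomly spawns BP_SewerslideBomb or BP_FlyingEnemy at its own transform, printing validity for debugging.
; After each batch, a rising increment enlarges the next one.
; A third switch branch duplicates the flying enemy but is unreachable with the random range used.
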(event Custom|SpawnEnemy
  (bind _returnvalue (Transformation|GetActorTransform))
  (for _index (range 0 (- (Variables|Default|GetEnemySpawned) 1))
    (switch int (Math|Random|RandomInteger 2)
      (:0
        (bind _returnvalue_2 (Game|SpawnActorfromClass "/Game/AI/Actors/BP_SewerslideBomb.BP_SewerslideBomb_C" _returnvalue "AdjustIfPossibleButAlwaysSpawn" "MultiplyWithRoot" 0 0))
        (Utilities|IsValid _returnvalue_2
          (:Is%20Valid
            (Development|PrintString "yes" :!label _label))
          (:Is%20Not%20Valid
            (Development|PrintString "no" :!label _label_2))))
      (:1
        (bind _returnvalue_3 (Game|SpawnActorfromClass "/Game/AI/Actors/BP_FlyingEnemy.BP_FlyingEnemy_C" _returnvalue "AdjustIfPossibleButAlwaysSpawn" "MultiplyWithRoot" 0 0))
        (Utilities|IsValid _returnvalue_3
          (:Is%20Valid
            (goto _label))
          (:Is%20Not%20Valid
            (goto _label_2))))
      (:2
        (bind _returnvalue_4 (Game|SpawnActorfromClass "/Game/AI/Actors/BP_FlyingEnemy.BP_FlyingEnemy_C" (Transformation|GetActorTransform) "AdjustIfPossibleButAlwaysSpawn" "MultiplyWithRoot" 0 0))
        (Utilities|IsValid _returnvalue_4
          (:Is%20Valid
            (goto _label))
          (:Is%20Not%20Valid
            (goto _label_2))))))
  (Math|Integer|IncrementInt (Variables|Default|GetEnemyIncrement)
    (:%20%20
      (Variables|Default|SetEnemySpawned (+ (Variables|Default|GetEnemySpawned) (Variables|Default|GetEnemyIncrement))))))

(event EventBeginPlay
  (bind _asbp_first_person_game_mode (Utilities|Casting|CastToBP_FirstPersonGameMode (Game|GetGameMode)))
  (EventDispatchers|BindEventtoRespawnEnemy _asbp_first_person_game_mode (delegate Custom|SpawnEnemy)))

(fn ConstructionScript)