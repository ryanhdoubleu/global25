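; BP_BasicAIParent is the base enemy character, with health, an arc jump and an empty Attack event for children.
; It increments the game mode's EnemiesLeft on BeginPlay, then decrements it and triggers a check when damage empties Health.
; JumptoDestination launches it along a suggested projectile arc aimed above the target.
; Death reveals a sphere, inverts gravity and launches the body upward before a delayed destroy.
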(event Custom|Attack)

(event EventJumptoDestination
  (params (Destination :type Vector :default "0, 0, 0"))
  (bind (_x _y _z) (Math|Vector|BreakVector Destination))
  (bind _outlaunchvelocity (Game|SuggestProjectileVelocityCustomArc (Transformation|GetActorLocation) (Math|Vector|MakeVector _x _y (+ _z 1.5e+02)) 0.0 0.5))
  (Character|LaunchCharacter _outlaunchvelocity true true))

(event EventDamageDealt
  (params (Damage :type Float%20%28double-precision%29))
  (bind _output_get (Variables|Default|SetHealth (- (Variables|Default|GetHealth) Damage)))
  (if (<= _output_get 0.0)
    (bind _asbp_first_person_game_mode (Utilities|Casting|CastToBP_FirstPersonGameMode (Game|GetGameMode)))
    (Math|Integer|DecrementInt (Variables|/Game/FirstPerson/Blueprints/BP_FirstPersonGameMode.BP_FirstPersonGameMode_C|GetEnemiesLeft _asbp_first_person_game_mode)
      (:%20%20
        (Default|CheckEnemyLeft _asbp_first_person_game_mode)
        (Rendering|SetVisibility (Variables|Default|GetSphere) true false)
        (Variables|/Script/Engine.CharacterMovementComponent|SetGravityScale (Variables|Character|GetCharacterMovement) -1.0)
        (Character|LaunchCharacter "0.000000,0.000000,1000.000000" false true)
        (Utilities|FlowControl|Delay 4.0)
        (Actor|DestroyActor)))))

(event EventBeginPlay
  (bind _asbp_first_person_game_mode (Utilities|Casting|CastToBP_FirstPersonGameMode (Game|GetGameMode)))
  (Math|Integer|IncrementInt (Variables|/Game/FirstPerson/Blueprints/BP_FirstPersonGameMode.BP_FirstPersonGameMode_C|GetEnemiesLeft _asbp_first_person_game_mode)))

(fn ConstructionScript)