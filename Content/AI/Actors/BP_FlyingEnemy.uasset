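; Flying AI enemy that registers itself in the first-person game mode's enemy count and fires projectiles from an arrow component when Attack is called.
; Construction sets its attack range and assigns the BT_FlyingAI_LOBOTOMIZED behavior tree.
; A looping fast timer spins the wings and smoothly rotates the actor toward its velocity, or toward the player when nearly stationary.
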(event Custom|RotationActivate
  (bind _wings (Variables|Default|Getwings))
  (bind _relativerotation (Variables|/Script/Engine.SceneComponent|GetRelativeRotation _wings))
  (CallFunction|Rotation)
  (Transformation|SetRelativeRotation _wings (Math|Rotator|MakeRotator (.roll _relativerotation) (.pitch _relativerotation) (+ (.yaw _relativerotation) 3.0)) false false))

(event EventBeginPlay
  (bind _returnvalue (Utilities|Time|SetTimerbyEvent (delegate Custom|RotationActivate) 0.01 true))
  (Variables|Default|SetTimerHandle _returnvalue)
  (bind _asbp_first_person_game_mode (Utilities|Casting|CastToBP_FirstPersonGameMode (Game|GetGameMode)))
  (Math|Integer|IncrementInt (Variables|/Game/FirstPerson/Blueprints/BP_FirstPersonGameMode.BP_FirstPersonGameMode_C|GetEnemiesLeft _asbp_first_person_game_mode)))

(event EventAttack
  (Game|SpawnActorfromClass "/Game/AI/AIToys/BP_ProjectileAI.BP_ProjectileAI_C" (Transformation|GetWorldTransform (Variables|Default|GetArrow1)) "AlwaysSpawn" "MultiplyWithRoot" 0 0))

(fn ConstructionScript
  (|CallParentFunction)
  (Variables|Default|SetAttackRange 1e+03)
  (Variables|Default|SetBehaviorTree "/Game/AI/BehaviourTrees/BT_FlyingAI_LOBOTOMIZED.BT_FlyingAI_LOBOTOMIZED"))

(fn Rotation
  (bind _charactermovement (Variables|Character|GetCharacterMovement))
  (bind _velocity (Variables|/Script/Engine.MovementComponent|GetVelocity _charactermovement))
  (bind _returnvalue (Math|Conversions|RotationFromXVector _velocity))
  (if (Utilities|Operators|EqualEqual :A _velocity :ErrorTolerance 5.0)
    (Transformation|SetActorRotation (Math|Interpolation|RInterpTo (Transformation|GetActorRotation) (Math|Rotator|FindLookatRotation (Transformation|GetActorLocation) (Transformation|GetActorLocation (Game|GetPlayerCharacter 0))) (Utilities|Time|GetWorldDeltaSeconds) 9.0))
    (else
      (Transformation|SetActorRotation (Math|Interpolation|RInterpTo (Transformation|GetActorRotation) (Math|Rotator|MakeRotator (.roll _returnvalue) (.pitch _returnvalue) (.yaw _returnvalue)) (Utilities|Time|GetWorldDeltaSeconds) 9.0)))))