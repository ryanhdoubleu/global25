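; BP_BubbleWand is a player melee weapon that deals damage to actors it touches during a swing.
; Swing plays a timeline that pitches the Cube mesh and flags CurrentlyAttacking, with a DoOnce blocking re-swings until it finishes.
; Box overlaps during an attack send bubble-wand and fixed damage messages to the other actor, throttled by a DoOnce and short delay.
; BeginPlay also stores all BP_BasicAIParent actors, though this graph never reads them.
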(event OnComponentBeginOverlap(Box)
  (params (OverlappedComponent :type Primitive%20Component%20Object%20Reference) (OtherActor :type Actor%20Object%20Reference) (OtherComp :type Primitive%20Component%20Object%20Reference) (OtherBodyIndex :type Integer) (bFromSweep :type Boolean) (SweepResult :type Hit%20Result%20Structure%20%28by%20ref%29))
  (if (Variables|Default|GetCurrentlyAttacking)
    (Utilities|FlowControl|DoOnce false :!label _label
      (:Completed
        (Class|BPIDamage|BubbleWandDamage(Message) OtherActor)
        (Class|BPIDamage|DamageDealt(Message) OtherActor 2e+01)
        (Utilities|FlowControl|Delay 0.2)
        (goto _label Reset)))
    (else
      (goto _label Reset))))

(event Custom|Swing
  (Utilities|FlowControl|DoOnce false :!label _label
    (:Completed
      (bind _newtrack_0 (Timeline|Timeline PlayFromStart)
        (:Update
          (Variables|Default|SetCurrentlyAttacking true)
          (Transformation|SetRelativeRotation (Variables|Default|GetCube) (Math|Rotator|MakeRotator 0.0 _newtrack_0 0.0) false false))
        (:Finished
          (Variables|Default|SetCurrentlyAttacking false)
          (goto _label Reset))))))

(event EventBeginPlay
  (bind _outactors (Actor|GetAllActorsOfClass "/Game/AI/Actors/BP_BasicAIParent.BP_BasicAIParent_C"))
  (Variables|Default|SetOut%20Actors _outactors))

(event Collision|EventActorBeginOverlap
  (params (OtherActor :type Actor%20Object%20Reference)))

(event EventTick
  (params (DeltaSeconds :type Float%20%28single-precision%29)))

(fn ConstructionScript)