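; BP_Bomb is a player weapon projectile that explodes on contact.
; A fast looping timer runs a small sphere trace around the bomb, ignoring the player pawn, and the first hit triggers detonation once.
; Detonation plays a boom, spawns BP_FartBubbles and messages damage to hits from a wider multi-sphere trace, skipping any matching DamagedActor, which is never set here.
; It then spawns a particle system and destroys itself.
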(event Custom|Collision
  (bind _returnvalue (Transformation|GetActorLocation))
  (bind _returnvalue_2 (Game|Player|GetPlayerPawn 0))
  (bind _returnvalue_3 (Transformation|GetActorLocation))
  (bind _returnvalue_4 (Transformation|GetActorLocation))
  (bind _array (Utilities|Array|MakeArray _returnvalue_2))
  (bind _returnvalue_5 (Collision|SphereTraceByChannel _returnvalue_4 _returnvalue_4 15.0 "TraceTypeQuery1" false _array "None"))
  (if _returnvalue_5
    (Utilities|FlowControl|DoOnce false
      (:Completed
        (Audio|PlaySoundatLocation "/Game/Sounds/Grenade_Boom.Grenade_Boom" _returnvalue "0, 0, 0" 1.0 1.0 0.0 0 0 0 0)
        (Game|SpawnActorfromClass "/Game/Player/weapons/BP_FartBubbles.BP_FartBubbles_C" (Math|Transform|MakeTransform _returnvalue) "Undefined" "MultiplyWithRoot" 0 0)
        (bind _outhits (Collision|MultiSphereTraceByChannel _returnvalue_3 _returnvalue_3 2e+02 "TraceTypeQuery1" false _array "None"))
        (for _array_element _outhits
          (if (!= (Variables|Default|GetDamaged%20actor) (.HitActor (Collision|BreakHitResult _array_element)))
            (Class|BPIDamage|DamageDealt(Message) (.HitActor (Collision|BreakHitResult _array_element)) 3e+01)))
        (Niagara|SpawnSystematLocation 0 (Transformation|GetActorLocation))
        (Actor|DestroyActor)))))

(event EventBeginPlay
  (Utilities|Time|SetTimerbyEvent (delegate Custom|Collision) 0.01 true))

(fn ConstructionScript)